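; Main menu HUD Blueprint that shows the menu on BeginPlay, sets the base sound mix and enables the mouse cursor.
; Widgets are reached through BPAllUMG references, and the settings button event swaps the main menu for the settings screen.
; Other events forward apply requests to the audio and display settings, and resolution and FPS limit choices to display settings.
; A ToDo marks the cursor setup for relocation to a custom controller.
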(event `self.ReceiveBeginPlay`
  (`GameplayStatics.SetBaseSoundMix` "/Game/EnableA/Game/Sounds/SoundMicher.SoundMicher")
  (`UserWidget.AddToViewport` (`/Game/EnableA/MainMenu/Core/BP_AllUMG.RefMainMenu` (`self.BP_AllUMG`)) 0)
  ;[1 1 1] ToDo: при добавлении собственного контроллера, поставить настройку в него, а эту удалить
  (set `PlayerController.bShowMouseCursor` true (`GameplayStatics.GetPlayerController` 0)))

(event `ButtonSettingsReleasedForHUD`
  (`Widget.RemoveFromParent` (`/Game/EnableA/MainMenu/Core/BP_AllUMG.RefMainMenu` (`self.BP_AllUMG`)))
  (`UserWidget.AddToViewport` (`/Game/EnableA/MainMenu/Core/BP_AllUMG.RefAllSettings` (`self.BP_AllUMG`)) 0))

(event `ButtonApplySettings`
  (bind _refallsettings (`/Game/EnableA/MainMenu/Core/BP_AllUMG.RefAllSettings` (`self.BP_AllUMG`)))
  (`/Game/EnableA/MainMenu/SubMenuSettings/SettingsAudio.Apply` (`/Game/EnableA/MainMenu/SubMenuSettings/AllSettings.SettingsAudio` _refallsettings))
  (`/Game/EnableA/MainMenu/SubMenuSettings/SettingsDisplay.Apply` (`/Game/EnableA/MainMenu/SubMenuSettings/AllSettings.SettingsDisplay` _refallsettings)))

(event `ScreenResolutionChoose`
  (params (IntX :type Integer) (IntY :type Integer))
  (`/Game/EnableA/MainMenu/SubMenuSettings/SettingsDisplay.ScreenResolytionChoose` (`/Game/EnableA/MainMenu/SubMenuSettings/AllSettings.SettingsDisplay` (`/Game/EnableA/MainMenu/Core/BP_AllUMG.RefAllSettings` (`self.BP_AllUMG`))) IntX IntY))

(event `EventFPS`
  (params (FPSLimit :type String))
  (`/Game/EnableA/MainMenu/SubMenuSettings/SettingsDisplay.FPS` (`/Game/EnableA/MainMenu/SubMenuSettings/AllSettings.SettingsDisplay` (`/Game/EnableA/MainMenu/Core/BP_AllUMG.RefAllSettings` (`self.BP_AllUMG`))) FPSLimit))

(fn `UserConstructionScript`)