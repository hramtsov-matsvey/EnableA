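; Player character for a top-down, cursor-aimed game, moved along world axes with WASD.
; Key events set direction flags and switch the mesh between looping jog and idle animations via PlayAnimation.
; Tick feeds the flags into HeroMovementBase as movement input and calls RotateHero, which yaws the mesh toward the cursor hit from BP_PlayerControllerPlay.
; The speed buff pickup logic is disabled; debug prints remain.
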(event `self.ReceiveBeginPlay`
  (set `CharacterMovementComponent.MaxWalkSpeed` (`self.Hero Movement Speed`) (`self.CharacterMovement`)))

(event `self.ReceiveTick`
  (params (DeltaSeconds :type "Float (single-precision)"))
  (`self.Rotate Hero`)
  (if (or (`self.W`) (`self.A`) (`self.S`) (`self.D`))
    (`self.HeroMovementBase` (`self.W`) (`self.A`) (`self.S`) (`self.D`))
    (else
      (`KismetSystemLibrary.PrintString` "don't move" true true (struct :`G` 0.66 :`B` 1.0 :`A` 1.0) 0.0))))

(event `Key|W`
  (params (Key :type "Key Structure"))
  (:`Pressed`
    ;[1 1 1] BaseAnimEvent
    (set `self.W` true)
    (if (not (or (`self.A`) (`self.S`) (`self.D`)))
      (`SkeletalMeshComponent.PlayAnimation` (`self.Mesh`) "/Game/MCO_Mocap_Basics/Animation/Mobility_Pro/In_Place/MOB1_Jog_F_IPC.MOB1_Jog_F_IPC" true :!label _label)))
  (:`Released`
    (set `self.W` false)
    (if (not (or (`self.A`) (`self.S`) (`self.D`)))
      (`SkeletalMeshComponent.PlayAnimation` (`self.Mesh`) "/Game/MCO_Mocap_Basics/Animation/Conversations/Root_Motion/Convo_01_Low_Key_Loop.Convo_01_Low_Key_Loop" true :!label _label_2))))

(event `InputAxis|MoveUpward`
  (params (AxisValue :type "Float (single-precision)")))

(event `Key|A`
  (params (Key :type "Key Structure"))
  (:`Pressed`
    ;[1 1 1] BaseAnimEvent
    (set `self.A` true)
    (if (not (or (`self.W`) (`self.S`) (`self.D`)))
      (goto _label)))
  (:`Released`
    (set `self.A` false)
    (if (not (or (`self.W`) (`self.S`) (`self.D`)))
      (goto _label_2))))

(event `InputAxis|MoveLeft`
  (params (AxisValue :type "Float (single-precision)")))

(event `Key|S`
  (params (Key :type "Key Structure"))
  (:`Pressed`
    ;[1 1 1] BaseAnimEvent
    (set `self.S` true)
    (if (not (or (`self.W`) (`self.A`) (`self.D`)))
      (goto _label)))
  (:`Released`
    (set `self.S` false)
    (if (not (or (`self.W`) (`self.A`) (`self.D`)))
      (goto _label_2))))

(event `Key|D`
  (params (Key :type "Key Structure"))
  (:`Pressed`
    ;[1 1 1] BaseAnimEvent
    (set `self.D` true)
    (if (not (or (`self.W`) (`self.A`) (`self.S`)))
      (goto _label)))
  (:`Released`
    (set `self.D` false)
    (if (not (or (`self.W`) (`self.A`) (`self.S`)))
      (goto _label_2))))

(event `PickUpSpeedBuff` :!enabledstate Disabled
  (params (SpeedBuff :type "Float (double-precision)") (LifetimeBuff :type "Float (double-precision)"))
  (bind _output_get (set `self.SpeedBuff` SpeedBuff :!enabledstate Disabled)))

(fn `HeroMovementBase`
  (params (W :type Boolean) (A :type Boolean) (S :type Boolean) (D :type Boolean))
  (if W
    (`PawnMovementComponent.AddInputVector` (`self.CharacterMovement`) (1.0 0.0 0.0) false))
  (if A
    (`PawnMovementComponent.AddInputVector` (`self.CharacterMovement`) (0.0 -1.0 0.0) false))
  (if S
    (`PawnMovementComponent.AddInputVector` (`self.CharacterMovement`) (-1.0 0.0 0.0) false))
  (if D
    (`PawnMovementComponent.AddInputVector` (`self.CharacterMovement`) (0.0 1.0 0.0) false))
  (`KismetSystemLibrary.PrintString` "moveing" true true (struct :`G` 0.66 :`B` 1.0 :`A` 1.0) 0.0))

(fn `Rotate Hero`
  (bind (_returnvalue_x _returnvalue_y) (`KismetMathLibrary.BreakVector` (`self.K2_GetActorLocation`)))
  (bind _asbp_player_controller_play (cast `/Game/EnableA/Core/GameCore/BP_PlayerControllerPlay` (`GameplayStatics.GetPlayerController` 0)))
  (bind _hitresult (`PlayerController.GetHitResultUnderCursorByChannel` _asbp_player_controller_play "TraceTypeQuery1" true))
  (if (`GameplayStatics.BreakHitResult` _hitresult)
    (bind (_returnvalue_roll _returnvalue_pitch _returnvalue_yaw) (`KismetMathLibrary.BreakRotator` (`KismetMathLibrary.FindLookAtRotation` (`KismetMathLibrary.MakeVector` _returnvalue_x _returnvalue_y) (`KismetMathLibrary.MakeVector` (.x (`.Location` (`GameplayStatics.BreakHitResult` _hitresult))) (.y (`.Location` (`GameplayStatics.BreakHitResult` _hitresult)))))))
    (`SceneComponent.K2_SetRelativeRotation` (`self.Mesh`) (`KismetMathLibrary.MakeRotator` 0.0 0.0 (+ _returnvalue_yaw -90.0)) false false)
    (else
      (`KismetSystemLibrary.PrintString` "false"))))

(fn `UserConstructionScript`)