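; Semi-automatic pistol weapon with magazine reload and an overheating mechanic.
; Fire gates shots with delays and runs a debug-drawn line trace along a randomly chosen spread variant that widens with heat; hits apply no damage yet.
; Each shot adds heat, while Tick updates the HUD overheat display, cools the weapon per frame and clamps heat at zero.
; The overheat burn effect is only a placeholder print.
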(event `self.ReceiveBeginPlay`
  ;[1 1 1 1 95] Это оружие стреляет одиночками с небольшим кд,
  (bind _asbp_hudin_game (cast `/Game/EnableA/Game/HUDInGame/BP_HUDInGame` (`PlayerController.GetHUD` (`GameplayStatics.GetPlayerController` 0)))
    (:`then`
      (`parent.ReceiveBeginPlay`)
      (`/Game/EnableA/Game/HUDInGame/ChildsInGameWidget/OverHeating/W_Overheating.SetPersentOverheating` (`/Game/EnableA/Game/HUDInGame/W_InGame.W_Overheating` (`/Game/EnableA/Game/HUDInGame/BPC_AllUMGInGame.RefWInGame` (`/Game/EnableA/Game/HUDInGame/BP_HUDInGame.BPC_AllUMGInGame` _asbp_hudin_game))) (`self.WeaponBurn`) :!label _label))
    (:`CastFailed`
      (`KismetSystemLibrary.PrintString` "cast fail \nBP_WeaponPistol1"))))

(event `self.ReceiveTick`
  (params (DeltaSeconds :type "Float (single-precision)"))
  ;[1 1 1 1 95] Это оружие стреляет одиночками с небольшим кд,
  (`|ExecutionSequence`
    (:`then_0`
      (goto _label))
    (:`then_1`
      (set `self.WeaponBurn` (- (`self.WeaponBurn`) 0.1))
      (if (< (`self.WeaponBurn`) 0.0)
        (set `self.WeaponBurn` 0.0))
      (if (> (`self.WeaponBurn`) 100.0)
        (`KismetSystemLibrary.PrintString` "перегрев включай эффект ожога на весь экран, пока перегрев не спадёт" true true (struct :`R` 1.0 :`G` 0.047766 :`A` 1.0) 0.0)))))

(event `/Game/EnableA/Game/InteractiveObjects/Weapon/BPI_WeaponFire.Fire`
  (params (HeroDamage :type "Float (single-precision)"))
  (bind (_returnvalue_x _returnvalue_y _returnvalue_z) (`KismetMathLibrary.BreakVector` (`self.GetActorForwardVector`)))
  (bind (_returnvalue_x_2 _returnvalue_y_2 _returnvalue_z_2) (`KismetMathLibrary.BreakVector` (`self.GetActorForwardVector`)))
  (bind (_returnvalue_x_3 _returnvalue_y_3 _returnvalue_z_3) (`KismetMathLibrary.BreakVector` (`self.GetActorForwardVector`)))
  (bind (_returnvalue_x_4 _returnvalue_y_4 _returnvalue_z_4) (`KismetMathLibrary.BreakVector` (`self.GetActorForwardVector`)))
  (bind (_returnvalue_x_5 _returnvalue_y_5 _returnvalue_z_5) (`KismetMathLibrary.BreakVector` (`self.GetActorForwardVector`)))
  (bind (_returnvalue_x_6 _returnvalue_y_6 _returnvalue_z_6) (`KismetMathLibrary.BreakVector` (`self.GetActorForwardVector`)))
  (bind _returnvalue (`KismetMathLibrary.RandomFloatInRange` 0.0 (`self.TimesDerivation`)))
  (bind _returnvalue_2 (`KismetMathLibrary.RandomFloatInRange` 0.0 (`self.TimesDerivation`)))
  (bind _returnvalue_3 (`KismetMathLibrary.RandomFloatInRange` 0.0 (`self.TimesDerivation`)))
  (bind _returnvalue_4 (`KismetMathLibrary.RandomFloatInRange` 0.0 (`self.TimesDerivation`)))
  (bind _returnvalue_5 (`SceneComponent.K2_GetComponentLocation` (`self.Arrow`)))
  (bind _returnvalue_6 (`SceneComponent.K2_GetComponentLocation` (`self.Arrow`)))
  (bind _returnvalue_7 (`SceneComponent.K2_GetComponentLocation` (`self.Arrow`)))
  (bind _returnvalue_8 (`SceneComponent.K2_GetComponentLocation` (`self.Arrow`)))
  (bind _returnvalue_9 (`SceneComponent.K2_GetComponentLocation` (`self.Arrow`)))
  (bind _returnvalue_10 (`SceneComponent.K2_GetComponentLocation` (`self.Arrow`)))
  (bind _returnvalue_11 (`KismetMathLibrary.RandomFloatInRange` 0.0 (`self.TimesDerivation`)))
  (bind _returnvalue_12 (`KismetMathLibrary.RandomFloatInRange` 0.0 (`self.TimesDerivation`)))
  ;[1 1 1 1 95] Это оружие стреляет одиночками с небольшим кд,
  ;;[1 1 1] Semi
  (if (`self.ReadyToShoot`)
    (set `self.ReadyToShoot` false)
    (if (== (`self.NumberOf Remaining AmmoInTheMagazine`) 0)
      (`KismetSystemLibrary.Delay` (`self.RemovalAndReloading`))
      (set `self.NumberOf Remaining AmmoInTheMagazine` (`self.MagazineCapacity`))
      (set `self.ReadyToShoot` true)
      (else
        (switch `int` (`KismetMathLibrary.RandomInteger` 5)
          (:`0`
            ;;[1 1 1] Логика деривации
            ;;;[1 1 1] Вариант 1
            (set `self.TimesDerivation` (- (/ (`self.WeaponBurn`) 300.0) (`self.Derivation `)))
            (`KismetSystemLibrary.LineTraceSingle` :`Start` _returnvalue_7 :`End` (+ (* (`KismetMathLibrary.MakeVector` (+ _returnvalue_x_3 _returnvalue_4) (+ _returnvalue_y_3 _returnvalue_4) _returnvalue_z_3) 1000.0) _returnvalue_7) :`TraceChannel` "TraceTypeQuery1" :`DrawDebugType` "Persistent"))
          (:`1`
            ;;;[1 1 1] Вариант2
            (set `self.TimesDerivation` (+ (`self.Derivation `) (/ (`self.WeaponBurn`) 300.0)))
            (`KismetSystemLibrary.LineTraceSingle` :`Start` _returnvalue_6 :`End` (+ (* (`KismetMathLibrary.MakeVector` (+ _returnvalue_x_4 _returnvalue_11) (+ _returnvalue_y_4 _returnvalue_11) _returnvalue_z_4) 1000.0) _returnvalue_6) :`TraceChannel` "TraceTypeQuery1" :`DrawDebugType` "Persistent"))
          (:`2`
            ;;;[1 1 1] Вариант3
            (set `self.TimesDerivation` (+ (`self.Derivation `) (/ (`self.WeaponBurn`) 300.0)))
            (`KismetSystemLibrary.LineTraceSingle` :`Start` _returnvalue_8 :`End` (+ (* (`KismetMathLibrary.MakeVector` (- _returnvalue_x_5 _returnvalue_12) (+ _returnvalue_y_5 _returnvalue_12) _returnvalue_z_5) 1000.0) _returnvalue_8) :`TraceChannel` "TraceTypeQuery1" :`DrawDebugType` "Persistent"))
          (:`3`
            ;;;[1 1 1] Вариант4
            (set `self.TimesDerivation` (+ (`self.Derivation `) (/ (`self.WeaponBurn`) 300.0)))
            (`KismetSystemLibrary.LineTraceSingle` :`Start` _returnvalue_9 :`End` (+ (* (`KismetMathLibrary.MakeVector` (+ _returnvalue_x_6 _returnvalue) (- _returnvalue_y_6 _returnvalue) _returnvalue_z_6) 1000.0) _returnvalue_9) :`TraceChannel` "TraceTypeQuery1" :`DrawDebugType` "Persistent"))
          (:`4`
            ;;;[1 1 1] Вариант 5
            (set `self.TimesDerivation` (+ (`self.Derivation `) (/ (`self.WeaponBurn`) 300.0)))
            (`KismetSystemLibrary.LineTraceSingle` :`Start` _returnvalue_10 :`End` (+ (* (`KismetMathLibrary.MakeVector` (- _returnvalue_x_2 _returnvalue_2) (- _returnvalue_y_2 _returnvalue_2) _returnvalue_z_2) 1000.0) _returnvalue_10) :`TraceChannel` "TraceTypeQuery1" :`DrawDebugType` "Persistent"))
          (:`5`
            ;;;[1 1 1] Вариант6
            (set `self.TimesDerivation` (- (/ (`self.WeaponBurn`) 300.0) (`self.Derivation `)))
            (`KismetSystemLibrary.LineTraceSingle` :`Start` _returnvalue_5 :`End` (+ (* (`KismetMathLibrary.MakeVector` (+ _returnvalue_x _returnvalue_3) (- _returnvalue_y _returnvalue_3) _returnvalue_z) 1000.0) _returnvalue_5) :`TraceChannel` "TraceTypeQuery1" :`DrawDebugType` "Persistent")))
        (set `self.WeaponBurn` (+ (`self.WeaponBurn`) (+ 8.0 (`self.WeaponBurnModificator`))))
        (`/Engine/EditorBlueprintResources/StandardMacros.DecrementInt` (`self.NumberOf Remaining AmmoInTheMagazine`)
          (:`  `
            (`KismetSystemLibrary.Delay` (`self.SpeedShooting`))
            (set `self.ReadyToShoot` true)))))))

(fn `UserConstructionScript`
  (`parent.UserConstructionScript`))